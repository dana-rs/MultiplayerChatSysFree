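; Game mode for the multiplayer chat system that hosts the game chatter component and hands joining players to it.
; BeginPlay adds and stores the component, then sets a ready flag.
; PostLogin polls that flag with a short delay loop, then passes the new player and default pawn class to the component.
; INFRefGameChatterAC exposes the stored component to other code.
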(event `self.ReceiveBeginPlay`
  (bind _returnvalue (`AddComponent|NODE_AddChatterInit_AC-0`))
  (set `self.GameChatterAC` _returnvalue)
  (set `self.IsReady?` true))

(event `self.K2_PostLogin`
  (params (NewPlayer :type "PlayerController Object Reference"))
  (if (`self.IsReady?`) :!label _label
    (`/Game/MultiplayerChatSys/Blueprint/Component/GameChatter_AC.FuncOnPostLogin` (`self.GameChatterAC`) NewPlayer (`self.DefaultPawnClass`))
    (else
      (`KismetSystemLibrary.Delay` 0.1)
      (goto _label))))

(fn `INFRefGameChatterAC`
  (returns (GameChatterAC :type "/Game/MultiplayerChatSys/Blueprint/Component/GameChatter_AC Object Reference"))
  (return (`self.GameChatterAC`)))

(fn `UserConstructionScript`)