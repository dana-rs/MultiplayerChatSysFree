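; Chatter_AC is a component in the multiplayer chat system that sets up each player on post-login.
; FuncOnPostLogin stores the given player and default pawn class and adds the player to an AllPlayers list.
; It then spawns that pawn at a default transform, owned by the player and adjusted for collisions, and has the player possess it.
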(fn `FuncOnPostLogin`
  (params (Player :type "PlayerController Object Reference") (DefaultPawn :type "Pawn Class Reference"))
  (locals (LocalPlayer :type "PlayerController Object Reference") (LocalDefaultPawn :type "Pawn Class Reference") (LocalPawn :type "Pawn Object Reference"))
  (set `local.LocalPlayer` Player)
  (set `local.LocalDefaultPawn` DefaultPawn)
  (`KismetArrayLibrary.Array_Add` (`self.AllPlayers`) (`local.LocalPlayer`))
  (bind _returnvalue (`|SpawnActorFromClass` (`local.LocalDefaultPawn`) (`self.DefaultSpawnTransform`) "AdjustIfPossibleButAlwaysSpawn" "OverrideRootScale" (`local.LocalPlayer`) null))
  (set `local.LocalPawn` _returnvalue)
  (`Controller.Possess` (`local.LocalPlayer`) (`local.LocalPawn`)))